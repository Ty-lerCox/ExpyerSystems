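; Town hall building actor that grants resources to player characters who enter its Resources component.
; On overlap, the server casts the other actor to FirstPersonCharacter and calls its IncreaseResourceRunOnServer with a fixed city, resource type and amount, independent of the hall's own City variable.
; Simple getters expose the building, city and food, stone and wood costs.
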(event OnComponentBeginOverlap(Resources)
  (params (OverlappedComponent :type Primitive%20Component%20Object%20Reference) (OtherActor :type Actor%20Object%20Reference) (OtherComp :type Primitive%20Component%20Object%20Reference) (OtherBodyIndex :type Integer) (bFromSweep :type Boolean) (SweepResult :type Hit%20Result%20Structure%20%28by%20ref%29))
  (Networking|SwitchHasAuthority
    (:Authority
      (bind _asfirst_person_character (Utilities|Casting|CastToFirstPersonCharacter OtherActor))
      (Default|IncreaseResourceRunonServer _asfirst_person_character "NewEnumerator4" "NewEnumerator0" 1))))

(event EventBeginPlay)

(event Collision|EventActorBeginOverlap
  (params (OtherActor :type Actor%20Object%20Reference)))

(event EventTick
  (params (DeltaSeconds :type Float%20%28single-precision%29)))

(fn ConstructionScript)

(fn GetBuilding
  (return (Variables|Default|GetBuilding)))

(fn GetCity
  (return (Variables|Default|GetCity)))

(fn GetFoodCost
  (return (Variables|Default|GetFood%20Cost)))

(fn GetStoneCost
  (return (Variables|Default|GetStone%20Cost)))

(fn GetWoodCost
  (return (Variables|Default|GetWood%20Cost)))