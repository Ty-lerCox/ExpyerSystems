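; House Blueprint, a building that exposes its identity and resource price through getter functions.
; The getters return its Building and City variables and a wood cost read from the Cost variable, while food and stone costs are zero.
; It has no behavior of its own, as the event graph and construction script are empty.
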(event EventBeginPlay)

(event Collision|EventActorBeginOverlap
  (params (OtherActor :type Actor%20Object%20Reference)))

(event EventTick
  (params (DeltaSeconds :type Float%20%28single-precision%29)))

(fn ConstructionScript)

(fn GetBuilding
  (return (Variables|Default|GetBuilding)))

(fn GetCity
  (return (Variables|Default|GetCity)))

(fn GetFoodCost
  (return 0))

(fn GetStoneCost
  (return 0))

(fn GetWoodCost
  (return (Variables|Default|GetCost)))