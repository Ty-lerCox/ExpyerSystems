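; Barracks building Blueprint that exposes its identity and resource costs, apparently for a city-building or strategy system.
; Five getter functions return its Building and City variables and its food, stone and wood costs.
; It has no gameplay logic of its own: the event graph holds only disabled default events and the construction script is empty.
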(event EventBeginPlay)

(event Collision|EventActorBeginOverlap
  (params (OtherActor :type Actor%20Object%20Reference)))

(event EventTick
  (params (DeltaSeconds :type Float%20%28single-precision%29)))

(fn ConstructionScript)

(fn GetBuilding
  (return (Variables|Default|GetBuilding)))

(fn GetCity
  (return (Variables|Default|GetCity)))

(fn GetFoodCost
  (return (Variables|Default|GetFood%20Cost)))

(fn GetStoneCost
  (return (Variables|Default|GetStone%20Cost)))

(fn GetWoodCost
  (return (Variables|Default|GetWood%20Cost)))