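; Base ACF player character Blueprint that handles movement input and gait switching.
; MoveForward and MoveRight axes add movement input relative to the control rotation.
; Sprint and Walk act as hold inputs that step LocomotionComp between adjacent locomotion states, each acting only from specific current states.
; Begin play, tick, overlap and the construction script are empty.
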(event EventBeginPlay)

(event Collision|EventActorBeginOverlap
  (params (OtherActor :type Actor%20Object%20Reference)))

(event EventTick
  (params (DeltaSeconds :type Float%20%28single-precision%29)))

(event Input|ActionEvents|InputActionSprint
  (params (Key :type Key%20Structure :default "None"))
  (bind _locomotioncomp (Variables|Default|GetLocomotionComp))
  (bind _returnvalue (Class|ACFLocomotionComponent|GetCurrentLocomotionState _locomotioncomp))
  (:Pressed
    (switch Utilities|FlowControl|Switch|SwitchonELocomotionState _returnvalue
      (:EJog
        (Class|ACFLocomotionComponent|AcceleratetoNextState _locomotioncomp))))
  (:Released
    (switch Utilities|FlowControl|Switch|SwitchonELocomotionState _returnvalue
      (:ESprint
        (Class|ACFLocomotionComponent|BraketoPreviousState _locomotioncomp)))))

(event Input|ActionEvents|InputActionWalk
  (params (Key :type Key%20Structure :default "None"))
  (bind _locomotioncomp (Variables|Default|GetLocomotionComp))
  (bind _returnvalue (Class|ACFLocomotionComponent|GetCurrentLocomotionState _locomotioncomp))
  (:Pressed
    (switch Utilities|FlowControl|Switch|SwitchonELocomotionState _returnvalue
      (:EIdle
        (Class|ACFLocomotionComponent|AcceleratetoNextState _locomotioncomp))
      (:EJog
        (Class|ACFLocomotionComponent|BraketoPreviousState _locomotioncomp))))
  (:Released
    (switch Utilities|FlowControl|Switch|SwitchonELocomotionState _returnvalue
      (:EWalk
        (Class|ACFLocomotionComponent|AcceleratetoNextState _locomotioncomp)))))

(event Input|AxisEvents|InputAxisMoveForward
  (params (AxisValue :type Float%20%28single-precision%29))
  (Pawn|Input|AddMovementInput (Math|Vector|GetForwardVector (Pawn|GetControlRotation :!class /Script/Engine.Pawn)) AxisValue false))

(event Input|AxisEvents|InputAxisMoveRight
  (params (AxisValue :type Float%20%28single-precision%29))
  (Pawn|Input|AddMovementInput (Math|Vector|GetRightVector (Pawn|GetControlRotation :!class /Script/Engine.Pawn)) AxisValue false))

(fn ConstructionScript)